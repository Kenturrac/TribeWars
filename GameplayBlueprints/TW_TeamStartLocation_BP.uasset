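; Team start location actor that holds a team assignment, a team artifact and a set of spawn point transforms.
; SetTeam stores the team and forwards it to the TeamArtifact.
; The construction script adds an arrow component at each SpawnPoints transform and records it in SpawnPointMeshes, giving every spawn point a visible marker.
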(event Custom|SetTeam
  (params (Team :type TW_Team_Enum%20Enum :default "NewEnumerator0"))
  (Variables|Default|SetTeam Team)
  (Default|SetTeam (Variables|Default|GetTeamArtifact) (Variables|Default|GetTeam)))

(fn ConstructionScript
  (Utilities|Array|Clear (Variables|Default|GetSpawnPointMeshes))
  (for _array_element (Variables|Default|GetSpawnPoints)
    (bind _returnvalue (AddComponent|AddArrowComponent false _array_element))
    (Utilities|Array|Add (Variables|Default|GetSpawnPointMeshes) _returnvalue)))